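; Mole actor for a whack-a-mole game that repeatedly pops up and down at random intervals.
; BeginSpawn loops by calling itself: it waits a random delay, plays the PopUpnDown level sequence, and opens a short IsActive window during the pop.
; Whacked snaps the sequence back to its first frame and pauses it, without stopping the spawn loop.
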(event Custom|BeginSpawn
  (Utilities|FlowControl|Delay (Math|Random|RandomFloatinRange 0.9 2.0))
  (Sequencer|Player|Play (Variables|/Script/ActorSequence.ActorSequenceComponent|GetSequencePlayer (Variables|Default|GetPopUpnDown)) :!class /Script/MovieScene.MovieSceneSequencePlayer)
  (Utilities|FlowControl|Delay 0.3)
  (Variables|Default|SetIsActive true)
  (Utilities|FlowControl|Delay 0.3)
  (Variables|Default|SetIsActive false)
  (Utilities|FlowControl|Delay 0.5)
  (CallFunction|BeginSpawn))

(event Custom|Whacked
  (bind _popupndown (Variables|Default|GetPopUpnDown))
  (bind _sequenceplayer (Variables|/Script/ActorSequence.ActorSequenceComponent|GetSequencePlayer _popupndown))
  (Components|Timeline|SetPlaybackPosition _sequenceplayer (Utilities|Struct|MakeMovieSceneSequencePlaybackParams (Utilities|Struct|MakeFrameTime (Utilities|Struct|MakeFrameNumber) 0.0) 0.0 "" "Frame" "Play"))
  (Sequencer|Player|Pause _sequenceplayer))

(event EventBeginPlay)

(event Collision|EventActorBeginOverlap
  (params (OtherActor :type Actor%20Object%20Reference)))

(event EventTick
  (params (DeltaSeconds :type Float%20%28single-precision%29)))

(fn ConstructionScript)